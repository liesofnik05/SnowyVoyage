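; BP_PipeHandles is a puzzle actor where two specific handle actors are fitted to pipes to complete the GetHandles quest.
; Each trigger box reacts to its referenced handle by toggling the mounted handle's visibility, destroying the overlapping actor and removing its smoke.
; Box2 is deactivated on BeginPlay and toggled active when the first handle attaches.
; A counter reaching two marks ACPuzzleElement solved and completes the quest.
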(event OnComponentBeginOverlap(Box1)
  (params (OverlappedComponent :type Primitive%20Component%20Object%20Reference) (OtherActor :type Actor%20Object%20Reference) (OtherComp :type Primitive%20Component%20Object%20Reference) (OtherBodyIndex :type Integer) (bFromSweep :type Boolean) (SweepResult :type Hit%20Result%20Structure%20%28by%20ref%29))
  (if (== OtherActor (Variables|Default|GetIsHandle))
    (CallFunction|ToggleVisibilityHandle1)))

(event OnComponentBeginOverlap(Box2)
  (params (OverlappedComponent :type Primitive%20Component%20Object%20Reference) (OtherActor :type Actor%20Object%20Reference) (OtherComp :type Primitive%20Component%20Object%20Reference) (OtherBodyIndex :type Integer) (bFromSweep :type Boolean) (SweepResult :type Hit%20Result%20Structure%20%28by%20ref%29))
  (if (== OtherActor (Variables|Default|GetIsHandle2))
    (CallFunction|ToggleVisibilityHandle2)))

(event Custom|CheckAmount
  (if (== (Variables|Default|GetBothHandlesAttached) 2.0)
    (Default|SetPuzzleSolved (Variables|Default|GetAC_PuzzleElement) true)
    (CallFunction|CompleteQuest "GetHandles")))

(event Custom|ToggleVisibilityHandle1
  (Rendering|ToggleVisibility (Variables|Default|GetHandle01) false)
  (Actor|DestroyActor (Variables|Default|GetIsHandle))
  (Components|Activation|Deactivate (Variables|Default|GetBox1))
  (Components|Activation|ToggleActive (Variables|Default|GetBox2))
  (Components|DestroyComponent (Variables|Default|GetSmoke1))
  (Variables|Default|SetBothHandlesAttached (+ (Variables|Default|GetBothHandlesAttached) 1.0))
  (Utilities|String|LogString "Hello")
  (CallFunction|CheckAmount))

(event Custom|ToggleVisibilityHandle2
  (Rendering|ToggleVisibility (Variables|Default|GetHandle02) false)
  (Actor|DestroyActor (Variables|Default|GetIsHandle2))
  (Utilities|FlowControl|Delay 0.2)
  (Components|Activation|Deactivate (Variables|Default|GetBox2))
  (Components|DestroyComponent (Variables|Default|GetSmoke2))
  (Variables|Default|SetBothHandlesAttached (+ (Variables|Default|GetBothHandlesAttached) 1.0))
  (Utilities|String|LogString "Hello")
  (CallFunction|CheckAmount))

(event EventBeginPlay
  (Components|Activation|Deactivate (Variables|Default|GetBox2)))

(fn ConstructionScript)