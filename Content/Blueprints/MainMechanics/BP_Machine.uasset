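; BP_Machine is a puzzle machine that gets fueled with coal to complete the "GetCoal" quest.
; When its Box trigger overlaps the referenced coal actor, it calls AddFire.
; AddFire toggles the point light's visibility, destroys the coal, marks its ACPuzzleElement as solved and completes the quest.
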(event OnComponentBeginOverlap(Box)
  (params (OverlappedComponent :type Primitive%20Component%20Object%20Reference) (OtherActor :type Actor%20Object%20Reference) (OtherComp :type Primitive%20Component%20Object%20Reference) (OtherBodyIndex :type Integer) (bFromSweep :type Boolean) (SweepResult :type Hit%20Result%20Structure%20%28by%20ref%29))
  (if (== OtherActor (Variables|Default|GetIsCoal))
    (CallFunction|AddFire)))

(event Custom|AddFire
  (Rendering|ToggleVisibility (Variables|Default|GetPointLight) false)
  (Actor|DestroyActor (Variables|Default|GetIsCoal))
  (Default|SetPuzzleSolved (Variables|Default|GetAC_PuzzleElement) true)
  (CallFunction|CompleteQuest "GetCoal"))

(event EventBeginPlay)

(event Collision|EventActorBeginOverlap
  (params (OtherActor :type Actor%20Object%20Reference)))

(event EventTick
  (params (DeltaSeconds :type Float%20%28single-precision%29)))

(fn ConstructionScript)