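; Interactable item that opens an inspection view where the player can rotate, pan and zoom a copy of its mesh.
; Construction duplicates the mesh 1000 units below, rendered alone by a SceneCapture2D, with zoom done through capture FOV.
; Interacting shows the UI_Inspect widget, switches BP_FirstPersonPlayerController to the inspection input context and adds the item's quest once.
; Exiting resets the copy and restores default input.
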(event Custom|Update%20Mesh%20Zoom
  (params (Axis :type Float%20%28double-precision%29))
  (Variables|/Script/Engine.SceneCaptureComponent2D|SetFOVAngle (Variables|Default|GetSceneCaptureComponent2D) (Math|Float|Clamp(Float) (+ (Variables|/Script/Engine.SceneCaptureComponent2D|GetFOVAngle (Variables|Default|GetSceneCaptureComponent2D)) (* Axis -4.0)) 0.0 1.2e+02)))

(event Custom|Update%20Mesh%20Rotation
  (params (Vector%202D :type Vector%202D%20Structure))
  (bind (_x _y) (Math|Vector2D|BreakVector2D Vector%202D))
  ;[0.15 0.15 0.15 0.5] Rotate Mesh on Mouse
  (Transformation|SetRelativeRotation (Variables|Default|GetInspectable%20Mesh) (Math|Rotator|CombineRotators (Variables|/Script/Engine.SceneComponent|GetRelativeRotation (Variables|Default|GetInspectable%20Mesh)) (Math|Rotator|MakeRotator (* _y -5.0) 0.0 (* _x -5.0))) false false))

(event Custom|Update%20Mesh%20Location
  (params (Vector%202D :type Vector%202D%20Structure))
  (bind (_x _y) (Math|Vector2D|BreakVector2D Vector%202D))
  (bind _inspectable_default_position (Variables|Default|GetInspectable%20Default%20Position))
  (bind _location (Math|Transform|BreakTransform _inspectable_default_position))
  (bind (_x_2 _y_2 _z) (Math|Vector|BreakVector _location))
  (Transformation|SetRelativeLocation (Variables|Default|GetInspectable%20Mesh) (Math|Vector|MakeVector (Math|Float|Clamp(Float) (+ (.x (Variables|/Script/Engine.SceneComponent|GetRelativeLocation (Variables|Default|GetInspectable%20Mesh))) (* _x 3.0)) (- _x_2 5e+01) (+ _x_2 5e+01)) 0.0 (Math|Float|Clamp(Float) (+ (.z (Variables|/Script/Engine.SceneComponent|GetRelativeLocation (Variables|Default|GetInspectable%20Mesh))) (* _y 3.0)) (- _z 5e+01) (+ _z 5e+01))) false false))

(event Custom|Exit%20Inspection%20Mode
  (bind _returnvalue (Game|GetPlayerController 0))
  ;[0.15 0.15 0.15 0.5] Exit Inspection Mode
  (CallFunction|ResetInspectableMesh)
  (Rendering|SetVisibility (Variables|Default|GetSceneCaptureComponent2D) false false)
  (Development|SetHiddeninGame (Variables|Default|GetInspectable%20Mesh) true false)
  (Widget|RemovefromParent (Variables|Default|GetInspect%20UI))
  (Variables|/Script/Engine.PlayerController|SetbShowMouseCursor _returnvalue false)
  (Input|SetInputModeGameOnly _returnvalue false)
  (bind _asbp_first_person_player_controller (Utilities|Casting|CastToBP_FirstPersonPlayerController (Game|GetPlayerController 0)))
  (Default|UpdateInputMapContext _asbp_first_person_player_controller "/Game/Input/IMC_Default.IMC_Default"))

(event Custom|Reset%20Inspectable%20Mesh
  ;[0.15 0.15 0.15 0.5] Exit Inspection Mode
  (Transformation|SetRelativeTransform (Variables|Default|GetInspectable%20Mesh) (Variables|Default|GetInspectable%20Default%20Position) false false)
  (Variables|/Script/Engine.SceneCaptureComponent2D|SetFOVAngle (Variables|Default|GetSceneCaptureComponent2D) 5e+01)
  (Class|SceneCaptureComponent|SetCaptureSortPriority (Variables|Default|GetSceneCaptureComponent2D) 1))

(event EventBeginPlay)

(event Collision|EventActorBeginOverlap
  (params (OtherActor :type Actor%20Object%20Reference)))

(event EventTick
  (params (DeltaSeconds :type Float%20%28single-precision%29)))

(event EventOnInteract
  (params (Component :type Primitive%20Component%20Object%20Reference))
  (bind _returnvalue (Game|GetPlayerController 0))
  (bind _scenecapturecomponent2d (Variables|Default|GetSceneCaptureComponent2D))
  (Class|SceneCaptureComponent|SetCaptureSortPriority _scenecapturecomponent2d)
  (Rendering|SetVisibility _scenecapturecomponent2d true false)
  (Development|SetHiddeninGame (Variables|Default|GetInspectable%20Mesh) false false)
  (bind _returnvalue_2 (UserInterface|CreateWidget "/Game/Blueprints/MainMechanics/InspectObjects/UI_Inspect.UI_Inspect_C"))
  (bind _output_get (Variables|Default|SetInspect%20UI _returnvalue_2))
  (UserInterface|Viewport|AddtoViewport _output_get 0)
  (Variables|/Script/Engine.PlayerController|SetbShowMouseCursor _returnvalue true)
  (Input|SetInputModeGameandUI _returnvalue 0 "DoNotLock" false false)
  (bind _asbp_first_person_player_controller (Utilities|Casting|CastToBP_FirstPersonPlayerController (Game|GetPlayerController 0)))
  (Default|UpdateInputMapContext _asbp_first_person_player_controller "/Game/Input/IMC_Inspection.IMC_Inspection")
  (bind _output_get_2 (Variables|/Game/FirstPerson/Blueprints/BP_FirstPersonPlayerController.BP_FirstPersonPlayerController_C|SetInspectable%20BP _asbp_first_person_player_controller self))
  (Class|BPIInteractable|InteractTriggerQuest(Message) _output_get_2 true))

(event EventOnInteractHighlight)

(fn ConstructionScript
  (bind _inspectable_mesh (Variables|Default|GetInspectable%20Mesh))
  (bind _scenecapturecomponent2d (Variables|Default|GetSceneCaptureComponent2D))
  (bind _relativelocation (Variables|/Script/Engine.SceneComponent|GetRelativeLocation _scenecapturecomponent2d))
  (bind _relativelocation_2 (Variables|/Script/Engine.SceneComponent|GetRelativeLocation _inspectable_mesh))
  (Rendering|SceneCapture|ShowOnlyComponent (Variables|Default|GetSceneCaptureComponent2D) (Variables|Default|GetInspectable%20Mesh))
  (Components|StaticMesh|SetStaticMesh (Variables|Default|GetInspectable%20Mesh) (Variables|/Script/Engine.StaticMeshComponent|GetStaticMesh (Variables|Default|GetInteractable%20Mesh)))
  (Transformation|SetRelativeTransform (Variables|Default|GetInspectable%20Mesh) (Transformation|GetRelativeTransform (Variables|Default|GetInteractable%20Mesh)) false false)
  (Transformation|SetRelativeLocation _inspectable_mesh (Math|Vector|MakeVector (.x _relativelocation_2) (.y _relativelocation_2) -1e+03) false false)
  (Transformation|SetRelativeLocation _scenecapturecomponent2d (Math|Vector|MakeVector (.x _relativelocation) (.y _relativelocation) -1e+03) false false)
  (Variables|Default|SetInspectable%20Default%20Position (Transformation|GetRelativeTransform (Variables|Default|GetInspectable%20Mesh))))

(fn GetInteractionInfo
  (return "Inspect"))

(fn InteractTriggerQuest
  (params (OnInteractionCompleted :type Boolean))
  (if OnInteractionCompleted
    (Utilities|FlowControl|DoOnce false
      (:Completed
        (CallFunction|AddQuest (Variables|Default|GetQuestToItem))
        (return)))))