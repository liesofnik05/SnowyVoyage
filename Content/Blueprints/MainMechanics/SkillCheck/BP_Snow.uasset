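; BP_Snow is an interactable snow pile that the player shovels through a bar skill check.
; Interacting opens UI_BarSkillCheck and switches to Game-and-UI input with the IMC_Solve mapping context.
; Each RemoveSnowPortion call decrements the layer count, lowers the mesh and plays a dig sound.
; At zero layers, completion removes the widget and restores game-only input and the default mapping, leaving the actor in place.
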(event Custom|RemoveSnowPortion
  (Utilities|FlowControl|Sequence
    (:then_0
      (Math|Integer|DecrementInt (Variables|Default|GetSnowLayer)
        (:%20%20
          (Transformation|SetRelativeLocation (Variables|Default|GetStaticMesh) (- (Variables|/Script/Engine.SceneComponent|GetRelativeLocation (Variables|Default|GetStaticMesh)) "0.000000,0.000000,10.000000") false false)
          (Audio|PlaySound2D "/Game/Audio/Prototype/S_SnowDig.S_SnowDig" 1.0 1.0 0.0 0 0))))
    (:then_1
      (if (<= (Variables|Default|GetSnowLayer) 0)
        (CallFunction|OnCompleted)))))

(event Custom|OnCompleted
  (bind _skillcheckref (Variables|Default|GetSkillCheckRef)
    (:then
      (Widget|RemovefromParent _skillcheckref)
      (Variables|Default|SetSkillCheckRef 0)
      (Input|SetInputModeGameOnly (Game|GetPlayerController 0) false)
      (bind _asbp_first_person_player_controller (Utilities|Casting|CastToBP_FirstPersonPlayerController (Game|GetPlayerController 0)))
      (Default|UpdateInputMapContext _asbp_first_person_player_controller "/Game/Input/IMC_Default.IMC_Default"))
    (:else)))

(event EventBeginPlay)

(event Collision|EventActorBeginOverlap
  (params (OtherActor :type Actor%20Object%20Reference)))

(event EventTick
  (params (DeltaSeconds :type Float%20%28single-precision%29)))

(event EventOnInteract
  (bind _returnvalue (UserInterface|CreateWidget "/Game/Blueprints/MainMechanics/SkillCheck/SkillCheck_Bar/UI_BarSkillCheck.UI_BarSkillCheck_C"))
  (bind _output_get (Variables|Default|SetSkillCheckRef _returnvalue))
  (UserInterface|Viewport|AddtoViewport _output_get 0)
  (Input|SetInputModeGameandUI (Game|GetPlayerController 0) 0 "DoNotLock" true false)
  (bind _asbp_first_person_player_controller (Utilities|Casting|CastToBP_FirstPersonPlayerController (Game|GetPlayerController 0)))
  (Default|UpdateInputMapContext _asbp_first_person_player_controller "/Game/Input/IMC_Solve.IMC_Solve"))

(fn ConstructionScript)

(fn GetInteractionInfo
  (return "Shovel"))