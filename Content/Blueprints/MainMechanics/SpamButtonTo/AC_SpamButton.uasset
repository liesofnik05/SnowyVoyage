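; Actor component for a button-mashing challenge that shows a progress bar and reports success or failure.
; Each press of the first key mapped to IA_Spam advances the bar toward a randomized target, which completes the task.
; It fails if no progress exists after four seconds, or when a retriggerable delay, restarted by any key release, expires.
; Either outcome removes the widget and destroys the component.
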(event Custom|Press%20Key
  (Variables|Default|SetAmountPressed (Math|Float|Clamp(Float) (+ (Variables|Default|GetAmountPressed) 1.0) 0.0 (Variables|Default|GetNeededAmount)))
  (Progress|SetPercent (Variables|/Game/Blueprints/MainMechanics/SpamButtonTo/UI_SpamButton.UI_SpamButton_C|GetSpamBar (Variables|Default|GetWidgetRef)) (/ (Variables|Default|GetAmountPressed) (Variables|Default|GetNeededAmount)))
  (if (== (Variables|Default|GetAmountPressed) (Variables|Default|GetNeededAmount))
    (Default|CallCompleted true)
    (CallFunction|Destroy)))

(event Custom|ReleaseKey
  (Utilities|FlowControl|RetriggerableDelay 0.8)
  (CallFunction|OnFailed))

(event Custom|Destroy
  (bind _widgetref (Variables|Default|GetWidgetRef)
    (:then
      (Widget|RemovefromParent _widgetref))
    (:else
      _))
  (Components|DestroyComponent))

(event Custom|OnFailed
  (Variables|Default|SetAmountPressed 0.0)
  (Progress|SetPercent (Variables|/Game/Blueprints/MainMechanics/SpamButtonTo/UI_SpamButton.UI_SpamButton_C|GetSpamBar (Variables|Default|GetWidgetRef)) (/ (Variables|Default|GetAmountPressed) (Variables|Default|GetNeededAmount)))
  (Default|CallCompleted false)
  (CallFunction|Destroy))

(event EventBeginPlay
  (bind _returnvalue (UserInterface|CreateWidget "/Game/Blueprints/MainMechanics/SpamButtonTo/UI_SpamButton.UI_SpamButton_C"))
  (Variables|Default|SetWidgetRef _returnvalue)
  (UserInterface|Viewport|AddtoViewport (Variables|Default|GetWidgetRef) 0)
  (Variables|Default|SetNeededAmount (Math|Random|RandomFloatinRange 1e+01 15.0))
  (Variables|Default|SetKeyPressed (Utilities|Array|Get(acopy) (Class|EnhancedInputSubsystemInterface|QueryKeysMappedtoAction (PlayerController|LocalPlayerSubsystems|GetEnhancedInputLocalPlayerSubsystem (Game|GetPlayerController 0)) "/Game/Input/Actions/IA_Spam.IA_Spam")))
  (Progress|SetPercent (Variables|/Game/Blueprints/MainMechanics/SpamButtonTo/UI_SpamButton.UI_SpamButton_C|GetSpamBar (Variables|Default|GetWidgetRef)) (/ (Variables|Default|GetAmountPressed) (Variables|Default|GetNeededAmount)))
  ;[0.15 0.15 0.15 0.5] If task not completed in 4 seconds, it fails
  (Utilities|FlowControl|Delay 4.0)
  (Utilities|IsValid self
    (:Is%20Valid
      (if (<= (Variables|Default|GetAmountPressed) 0.0)
        (CallFunction|OnFailed)))))

(event EventTick
  (params (DeltaSeconds :type Float%20%28single-precision%29)))

(event Input|KeyboardEvents|AnyKey
  (params (Key :type Key%20Structure :default "None"))
  (:Pressed
    (if (== Key (Variables|Default|GetKeyPressed))
      (CallFunction|PressKey)))
  (:Released
    (CallFunction|ReleaseKey)))

(fn UpdateProgressBar
  (Progress|SetPercent (Variables|/Game/Blueprints/MainMechanics/SpamButtonTo/UI_SpamButton.UI_SpamButton_C|GetSpamBar (Variables|Default|GetWidgetRef)) (/ (Variables|Default|GetAmountPressed) (Variables|Default|GetNeededAmount)))
  (return))

(fn GetInteractionInfo
  (return ""))