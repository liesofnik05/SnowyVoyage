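; BP_Drawer is an interactable drawer unit that slides a drawer open or closed, with a fixed "Open Drawer" prompt.
; Interacting with any component except the main body calls OpenDrawer, which always moves MDrawer03 regardless of the component hit.
; A timeline lerps its relative Y, playing forward or in reverse based on its current position.
; A DrawerOpening flag blocks re-triggering mid-motion, though the sound plays on every call; the quest trigger hook is empty.
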(event Custom|OpenDrawer
  (params (Component :type Primitive%20Component%20Object%20Reference))
  (bind _m_drawer03 (Variables|Default|GetM_Drawer03))
  (bind _relativelocation (Variables|/Script/Engine.SceneComponent|GetRelativeLocation _m_drawer03))
  (Audio|PlaySound2D "/Game/Audio/Prototype/S_DrawerOpening.S_DrawerOpening" 1.0 1.0 0.0 0 0)
  (if (not (Variables|Default|GetDrawerOpening))
    (Variables|Default|SetDrawerOpening true)
    (if (not (> (.y _relativelocation) 39.0))
      (bind _alpha (Timeline|OpenDrawer_TL PlayFromStart)
        (:Update
          (Transformation|SetRelativeLocation (Variables|Default|GetM_Drawer03) (Math|Vector|MakeVector (.x _relativelocation) (Math|Float|Lerp 6.0 6e+01 _alpha) (.z _relativelocation)) false false))
        (:Finished
          (Variables|Default|SetDrawerOpening false)))
      (else
        (Timeline|OpenDrawer_TL ReverseFromEnd)))))

(event EventOnInteract
  (params (Component :type Primitive%20Component%20Object%20Reference))
  (if (not (Utilities|Enum|Equal(Enum) (Utilities|GetObjectName Component) (Utilities|GetObjectName (Variables|Default|GetM_DrawerMainBody))))
    (CallFunction|OpenDrawer Component)))

(fn ConstructionScript)

(fn GetInteractionInfo
  (return "Open Drawer"))

(fn InteractTriggerQuest
  (params (OnInteractionCompleted :type Boolean))
  (return))