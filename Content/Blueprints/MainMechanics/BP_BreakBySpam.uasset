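; BP_BreakBySpam is a puzzle actor solved by rapidly spamming an input while the player stands in its trigger box.
; Overlap by the first-person character enables input and shows a UI_SpamButton widget, both removed on exit.
; IA_Spam presses increment a counter that updates the widget and marks ACPuzzleElement solved upon reaching the required count.
; A retriggerable delay after release resets the count and the solved state when spamming pauses.
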(event OnComponentBeginOverlap(Box_Collision)
  (params (OverlappedComponent :type Primitive%20Component%20Object%20Reference) (OtherActor :type Actor%20Object%20Reference) (OtherComp :type Primitive%20Component%20Object%20Reference) (OtherBodyIndex :type Integer) (bFromSweep :type Boolean) (SweepResult :type Hit%20Result%20Structure%20%28by%20ref%29))
  (Utilities|Casting|CastToBP_FirstPersonCharacter OtherActor)
  (Input|EnableInput (Game|GetPlayerController 0))
  (bind _returnvalue (UserInterface|CreateWidget "/Game/Blueprints/MainMechanics/UI_SpamButton.UI_SpamButton_C"))
  (bind _output_get (Variables|Default|SetWidgetRef _returnvalue))
  (UserInterface|Viewport|AddtoViewport _output_get 0)
  (Variables|/Game/Blueprints/MainMechanics/UI_SpamButton.UI_SpamButton_C|SetPresses%20Needed _output_get (Variables|Default|GetPresses%20Required)))

(event OnComponentEndOverlap(Box_Collision)
  (params (OverlappedComponent :type Primitive%20Component%20Object%20Reference) (OtherActor :type Actor%20Object%20Reference) (OtherComp :type Primitive%20Component%20Object%20Reference) (OtherBodyIndex :type Integer))
  (Utilities|Casting|CastToBP_FirstPersonCharacter OtherActor)
  (Input|DisableInput (Game|GetPlayerController 0))
  (Widget|RemovefromParent (stale OnComponentBeginOverlap(Box_Collision) _returnvalue)))

(event Input|EnhancedActionEvents|EnhancedInputActionIA_Spam
  (params (ActionValue :type Boolean) (ElapsedSeconds :type Float%20%28double-precision%29) (TriggeredSeconds :type Float%20%28double-precision%29) (InputAction :type Input%20Action%20Object%20Reference :default "/Game/Input/Actions/IA_Spam.IA_Spam"))
  (:Triggered
    (bind _result (Math|Float|IncrementFloat (Variables|Default|GetPressed%20Amount))
      (:%20%20
        (bind _output_get (Variables|Default|SetPressed%20Amount _result))
        (if (== _output_get (Variables|Default|GetPresses%20Required))
          (Default|SetPuzzleSolved (Variables|Default|GetAC_PuzzleElement) true)
          (else
            (Variables|/Game/Blueprints/MainMechanics/UI_SpamButton.UI_SpamButton_C|SetAmount%20Pressed (Variables|Default|GetWidgetRef) (stale _output_get_2) :!label _label)
            (Default|SetPuzzleSolved (Variables|Default|GetAC_PuzzleElement) false))))))
  (:Completed
    (Utilities|FlowControl|RetriggerableDelay 0.4)
    (bind _output_get_2 (Variables|Default|SetPressed%20Amount 0.0))
    (goto _label)))

(event EventBeginPlay)

(event Collision|EventActorBeginOverlap
  (params (OtherActor :type Actor%20Object%20Reference)))

(event EventTick
  (params (DeltaSeconds :type Float%20%28single-precision%29)))

(fn ConstructionScript)