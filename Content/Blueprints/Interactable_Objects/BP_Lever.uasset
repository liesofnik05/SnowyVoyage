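; BP_Lever is an interactable lever that shows "Crank" as its interaction info.
; On interact it enables actor collision and plays the LeverAnimation timeline, which lerps the relative yaw of LeverRoot through a very small angle.
; Logic to toggle the solved state of its ACPuzzleElement is present but unconnected, so interacting does not change puzzle state.
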(event EventBeginPlay)

(event Collision|EventActorBeginOverlap
  (params (OtherActor :type Actor%20Object%20Reference)))

(event EventTick
  (params (DeltaSeconds :type Float%20%28single-precision%29)))

(event EventOnInteract
  (Collision|SetActorEnableCollision true)
  (bind _value (Timeline|Lever%20Animation Play)
    (:Update
      (Transformation|SetRelativeRotation (Variables|Default|GetLever_Root) (Math|Rotator|MakeRotator 0.0 0.0 (Math|Float|Lerp 0.0 -0.2 _value)) false false))))

(fn ConstructionScript)

(fn GetInteractionInfo
  (return "Crank"))