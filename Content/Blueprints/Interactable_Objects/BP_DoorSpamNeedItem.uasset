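; Interactable door that the player breaks open with a button-spam minigame once a linked puzzle actor is solved.
; A puzzle-element component event sets the crowbar flag; interacting without it only plays a locked sound, while unsolving closes the door.
; With the flag, interacting adds a spam-button component whose success swings the door open via a timeline and clears the prompt.
; Quest completion logic exists but is never executed.
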(event Custom|Open
  (Audio|PlaySound2D "/Game/Audio/Prototype/S_DoorOpen.S_DoorOpen" 1.0 1.0 0.0 0 0)
  (bind (_direction _value) (Timeline|Door%20Animation Play)
    (:Update
      (Transformation|SetRelativeRotation (Variables|Default|GetDoor%20Root) (Math|Rotator|MakeRotator 0.0 0.0 (Math|Float|Lerp 0.0 -9e+01 _value)) false false))))

(event Custom|Close
  (bind (_direction _value) (Timeline|Door%20Animation Reverse)
    (:Update
      (Transformation|SetRelativeRotation (Variables|Default|GetDoor%20Root) (Math|Rotator|MakeRotator 0.0 0.0 (Math|Float|Lerp 0.0 -9e+01 _value)) false false))))

(event Custom|TriggerMinigame
  (Input|EnableInput (Game|GetPlayerController 0))
  (bind _returnvalue (AddComponent|AddACSpamButton))
  (EventDispatchers|BindEventtoCompleted _returnvalue (delegate Custom|On%20Completed)))

(event Custom|On%20Completed
  (params (Success :type Boolean))
  (if Success
    (CallFunction|Open)
    (Variables|Default|SetTaskDone true)
    (else
      (CallFunction|Close)
      (Variables|Default|SetTaskDone false)))
  (Input|DisableInput (Game|GetPlayerController 0)))

(event Custom|OnSolvedChanged
  (params (is%20Solved :type Boolean))
  (if is%20Solved
    (if (Variables|Default|GetOpens%20Just%20Once)
      (EventDispatchers|UnbindEventfromOnSolvedChanged (Actor|GetComponentbyClass (Variables|Default|GetPuzzleActor) "/Game/Blueprints/Interaction/AC_PuzzleElement.AC_PuzzleElement_C") (delegate Custom|OnSolvedChanged)))
    (Variables|Default|SetGotCrowbar true)
    (else
      (CallFunction|Close)
      (Variables|Default|SetGotCrowbar false))))

(event EventBeginPlay
  (bind _puzzleactor (Variables|Default|GetPuzzleActor)
    (:then
      (Utilities|IsValid (Actor|GetComponentbyClass _puzzleactor "/Game/Blueprints/Interaction/AC_PuzzleElement.AC_PuzzleElement_C")
        (:Is%20Valid
          (EventDispatchers|BindEventtoOnSolvedChanged (Actor|GetComponentbyClass _puzzleactor "/Game/Blueprints/Interaction/AC_PuzzleElement.AC_PuzzleElement_C") (delegate Custom|OnSolvedChanged)))))
    (:else)))

(event Collision|EventActorBeginOverlap
  (params (OtherActor :type Actor%20Object%20Reference)))

(event EventTick
  (params (DeltaSeconds :type Float%20%28single-precision%29)))

(event EventOnInteract
  (if (Variables|Default|GetGotCrowbar)
    (CallFunction|TriggerMinigame)
    (else
      (Audio|PlaySound2D "/Game/Audio/Prototype/S_DoorLocked.S_DoorLocked" 1.0 1.0 0.0 0 0))))

(fn ConstructionScript)

(fn GetInteractionInfo
  (if (Variables|Default|GetTaskDone)
    (return "")
    (else
      (return "Break Open"))))