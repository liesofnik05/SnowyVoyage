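; BP_DoorSpam is an interactable door that is broken open through a button-spam component, shown with a "Break Open" prompt.
; Interacting enables input and adds the spam component, whose completion result opens or closes the door before disabling input.
; Opening plays a sound and a timeline that swings DoorRoot's yaw, while closing reverses that timeline.
; Quest completion logic exists but is disconnected, so it never runs.
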(event Custom|Open
  (Audio|PlaySound2D "/Game/Audio/Prototype/S_DoorOpen.S_DoorOpen" 1.0 1.0 0.0 0 0)
  (bind (_direction _value) (Timeline|Door%20Animation Play)
    (:Update
      (Transformation|SetRelativeRotation (Variables|Default|GetDoor%20Root) (Math|Rotator|MakeRotator 0.0 0.0 (Math|Float|Lerp 0.0 -9e+01 _value)) false false))))

(event Custom|Close
  (bind (_direction _value) (Timeline|Door%20Animation Reverse)
    (:Update
      (Transformation|SetRelativeRotation (Variables|Default|GetDoor%20Root) (Math|Rotator|MakeRotator 0.0 0.0 (Math|Float|Lerp 0.0 -9e+01 _value)) false false))))

(event Custom|On%20Completed
  (params (Success :type Boolean))
  (if Success
    (CallFunction|Open)
    (else
      (CallFunction|Close)))
  (Input|DisableInput (Game|GetPlayerController 0)))

(event EventBeginPlay)

(event Collision|EventActorBeginOverlap
  (params (OtherActor :type Actor%20Object%20Reference)))

(event EventTick
  (params (DeltaSeconds :type Float%20%28single-precision%29)))

(event EventOnInteract
  (Input|EnableInput (Game|GetPlayerController 0))
  (bind _returnvalue (AddComponent|AddACSpamButton))
  (EventDispatchers|BindEventtoCompleted _returnvalue (delegate Custom|On%20Completed)))

(fn ConstructionScript)

(fn GetInteractionInfo
  (return "Break Open"))