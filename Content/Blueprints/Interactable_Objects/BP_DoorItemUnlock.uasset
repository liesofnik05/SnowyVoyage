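; Interactable door that stays locked until a linked puzzle actor reports solved.
; It listens to the actor's AC_PuzzleElement: solving unlocks it, unsolving closes and relocks it unless OpensJustOnce has unbound the listener.
; Interacting plays a locked sound, or swings DoorRoot open via a timeline and completes the hardcoded "OpenDoorA" quest.
; The CompletesQuest variable is only used in disconnected nodes.
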(event Custom|Open
  (bind (_direction _value) (Timeline|Door%20Animation Play)
    (:Update
      (Transformation|SetRelativeRotation (Variables|Default|GetDoor%20Root) (Math|Rotator|MakeRotator 0.0 0.0 (Math|Float|Lerp 0.0 -9e+01 _value)) false false))))

(event Custom|Close
  (bind (_direction _value) (Timeline|Door%20Animation Reverse)
    (:Update
      (Transformation|SetRelativeRotation (Variables|Default|GetDoor%20Root) (Math|Rotator|MakeRotator 0.0 0.0 (Math|Float|Lerp 0.0 -9e+01 _value)) false false))))

(event Custom|On%20Solved%20Changed_Event
  (params (is%20Solved :type Boolean))
  (if is%20Solved
    (if (Variables|Default|GetOpens%20Just%20Once)
      (EventDispatchers|UnbindEventfromOnSolvedChanged (Actor|GetComponentbyClass (Variables|Default|GetPuzzle%20Actor) "/Game/Blueprints/Interaction/AC_PuzzleElement.AC_PuzzleElement_C") (delegate Custom|On%20Solved%20Changed_Event)))
    (Variables|Default|SetTask%20Completed true)
    (Audio|PlaySound2D "/Game/Audio/Prototype/S_DoorUnlock.S_DoorUnlock" 1.0 1.0 0.0 0 0)
    (else
      (CallFunction|Close)
      (Variables|Default|SetTask%20Completed false))))

(event EventBeginPlay
  (bind _puzzle_actor (Variables|Default|GetPuzzle%20Actor)
    (:then
      (Utilities|IsValid (Actor|GetComponentbyClass _puzzle_actor "/Game/Blueprints/Interaction/AC_PuzzleElement.AC_PuzzleElement_C")
        (:Is%20Valid
          (EventDispatchers|AssignOnSolvedChanged (Actor|GetComponentbyClass _puzzle_actor "/Game/Blueprints/Interaction/AC_PuzzleElement.AC_PuzzleElement_C") (delegate Custom|On%20Solved%20Changed_Event)))))
    (:else)))

(event Collision|EventActorBeginOverlap
  (params (OtherActor :type Actor%20Object%20Reference)))

(event EventTick
  (params (DeltaSeconds :type Float%20%28single-precision%29)))

(event EventOnInteract
  (params (Component :type Primitive%20Component%20Object%20Reference))
  (if (Variables|Default|GetTask%20Completed)
    (CallFunction|Open)
    (CallFunction|CompleteQuest "OpenDoorA")
    (Audio|PlaySound2D "/Game/Audio/Prototype/S_DoorOpen.S_DoorOpen" 1.0 1.0 0.0 0 0)
    (Variables|Default|SetDoorOpened true)
    (else
      (Audio|PlaySound2D "/Game/Audio/Prototype/S_DoorLocked.S_DoorLocked" 1.0 1.0 0.0 0 0)
      (Variables|Default|SetDoorOpened false))))

(fn ConstructionScript)

(fn GetInteractionInfo
  (if (Variables|Default|GetDoorOpened)
    (return "")
    (else
      (return "Open"))))