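; BP_Button is an interactable puzzle button that shows a "Push" prompt and toggles its puzzle element's solved state.
; On interact it plays a click sound, disables collision, flips ACPuzzleElement's Solved state, and plays or reverses a timeline.
; The timeline slides ButtonRoot along local Z and re-enables collision when finished.
; The construction script derives the timeline's play rate from AnimationTimeInSeconds.
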(event EventBeginPlay)

(event Collision|EventActorBeginOverlap
  (params (OtherActor :type Actor%20Object%20Reference)))

(event EventTick
  (params (DeltaSeconds :type Float%20%28single-precision%29)))

(event EventOnInteract
  (bind _ac_puzzleelement (Variables|Default|GetAC_PuzzleElement))
  (Audio|PlaySoundatLocation "/Game/Audio/Prototyping/CUE_click1.CUE_click1" (Transformation|GetActorLocation) "0, 0, 0" 1.0 1.0 0.0 0 0 0 0)
  (Collision|SetActorEnableCollision false)
  (if (Variables|/Game/Blueprints/Interaction/AC_PuzzleElement.AC_PuzzleElement_C|GetSolved (Variables|Default|GetAC_PuzzleElement))
    ;[1 0.8496 0 0.5] Comment
    (Default|SetPuzzleSolved _ac_puzzleelement false)
    (bind _value (Timeline|Button%20Animation Reverse)
      (:Update
        (Transformation|SetRelativeLocation (Variables|Default|GetButton_Root) (Math|Vector|MakeVector 0.0 0.0 (Math|Float|Lerp 0.0 -5.0 _value)) false false))
      (:Finished
        (Collision|SetActorEnableCollision true)))
    (else
      (Default|SetPuzzleSolved _ac_puzzleelement true)
      (Timeline|Button%20Animation Play))))

(fn ConstructionScript
  (Components|Timeline|SetPlayRate (Variables|Default|GetButton%20Animation) (/ 1.0 (Variables|Default|GetAnimation%20Time%20in%20Seconds))))

(fn GetInteractionInfo
  (return "Push"))