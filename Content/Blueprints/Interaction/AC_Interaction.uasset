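; Interaction component that detects the interactable actor the player is looking at or pointing at and triggers it.
; Each tick it uses either a camera-forward line trace or a cursor hit test, chosen by a HUD view model flag.
; Hits implementing _BPI_Interactable are stored in that view model and switch the cursor to a hand; anything else clears both.
; IA_Interact sends the interact interface message to the stored actor.
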(event Custom|Set%20Current%20Interaction%20Actor
  (params (Current%20Interactable%20Actor :type Actor%20Object%20Reference))
  (bind _output_get (Variables|/Game/UI/VM_HUD.VM_HUD_C|SetCurrent%20Interactable%20Actor (CallFunction|GetHUDVM) Current%20Interactable%20Actor))
  (Variables|/Script/Engine.PlayerController|SetCurrentMouseCursor (Game|GetPlayerController 0) (select (Utilities|IsValid _output_get) "Hand" "Default")))

(event Input|EnhancedActionEvents|EnhancedInputActionIA_Interact
  (params (ActionValue :type Boolean) (ElapsedSeconds :type Float%20%28double-precision%29) (TriggeredSeconds :type Float%20%28double-precision%29) (InputAction :type Input%20Action%20Object%20Reference :default "/Game/Input/Actions/IA_Interact.IA_Interact"))
  (bind _current_interactable_actor (Variables|/Game/UI/VM_HUD.VM_HUD_C|GetCurrent%20Interactable%20Actor (CallFunction|GetHUDVM))
    (:then
      (Class|BPIInteractable|OnInteract(Message) _current_interactable_actor))
    (:else)))

(event EventBeginPlay)

(event EventTick
  (params (DeltaSeconds :type Float%20%28single-precision%29))
  (bind _returnvalue (Game|GetPlayerCameraManager 0))
  (bind _returnvalue_2 (Camera|GetCameraLocation _returnvalue))
  (bind _outhit (Collision|LineTraceByChannel _returnvalue_2 (+ _returnvalue_2 (* (Transformation|GetActorForwardVector _returnvalue) (Variables|Default|GetInteraction%20Range))) "TraceTypeQuery1" false 0 "None"))
  (if (.bBlockingHit (Collision|BreakHitResult (select (Variables|/Game/UI/VM_HUD.VM_HUD_C|GetUseMouseInteraction (CallFunction|GetHUDVM)) (.HitResult (Game|Player|GetHitResultUnderCursorbyChannel (Game|GetPlayerController 0) "TraceTypeQuery1" true)) _outhit)))
    (if (Utilities|DoesObjectImplementInterface (.HitActor (Collision|BreakHitResult (select (Variables|/Game/UI/VM_HUD.VM_HUD_C|GetUseMouseInteraction (CallFunction|GetHUDVM)) (.HitResult (Game|Player|GetHitResultUnderCursorbyChannel (Game|GetPlayerController 0) "TraceTypeQuery1" true)) _outhit))) "/Game/Blueprints/Interaction/_BPI_Interactable._BPI_Interactable_C")
      (CallFunction|SetCurrentInteractionActor (.HitActor (Collision|BreakHitResult (select (Variables|/Game/UI/VM_HUD.VM_HUD_C|GetUseMouseInteraction (CallFunction|GetHUDVM)) (.HitResult (Game|Player|GetHitResultUnderCursorbyChannel (Game|GetPlayerController 0) "TraceTypeQuery1" true)) _outhit))))
      (else
        (CallFunction|SetCurrentInteractionActor)))
    (else
      (CallFunction|SetCurrentInteractionActor))))