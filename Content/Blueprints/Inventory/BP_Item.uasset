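; BP_Item is an interactable pickup actor that adds its DT_Items row to the inventory when collected.
; The construction script looks up the row, caches it as ItemStruct and synchronously loads its soft-referenced mesh.
; Interacting hides the actor, disables collision, plays a sound, adds the row name to the inventory and marks ACPuzzleElement solved.
; GetInteractionInfo returns the item's display name.
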(event Custom|Collect
  (Rendering|SetActorHiddenInGame true)
  (Collision|SetActorEnableCollision false)
  (Audio|PlaySoundatLocation (Variables|Default|GetCollect%20Sound) "0, 0, 0" "0, 0, 0" 0.3 1.0 0.0 0 0 0 0)
  (CallFunction|AddItemtoInventory (.rowname (Variables|Default|GetItem))))

(event EventBeginPlay)

(event Collision|EventActorBeginOverlap
  (params (OtherActor :type Actor%20Object%20Reference)))

(event EventTick
  (params (DeltaSeconds :type Float%20%28single-precision%29)))

(event EventOnInteract
  (bind _ac_puzzleelement (Variables|Default|GetAC_PuzzleElement))
  (CallFunction|Collect)
  (if true
    (Default|SetPuzzleSolved _ac_puzzleelement true)
    (else
      (Default|SetPuzzleSolved _ac_puzzleelement false))))

(fn ConstructionScript
  (bind _returnvalue (Utilities|GetDataTableRow "/Game/Blueprints/Inventory/DT_Items.DT_Items" (.rowname (Variables|Default|GetItem)))
    (:then
      (bind _output_get (Variables|Default|Setitem%20Struct _returnvalue))
      (Utilities|LoadAssetBlocking (.mesh _output_get))
      (Components|StaticMesh|SetStaticMesh (Variables|Default|GetStaticMesh) (Utilities|ResolveSoftReference (.mesh _output_get))))))

(fn GetInteractionInfo
  (return (.displayname (Variables|Default|Getitem%20Struct))))