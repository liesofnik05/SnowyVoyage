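; Possessable crank puzzle master that the player interacts with and turns using keyboard move up/down input.
; On interact it stores the player's pawn, blends the view, possesses itself and pushes a keyboard puzzle widget; closing the widget restores the pawn.
; A timeline, rate-scaled by animation time, drives lever yaw forward or backward while input is held.
; Its solved check looks unfinished, as both branches set the puzzle unsolved.
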(event Custom|BP_OnWidgetDeactivated_Event
  (bind _returnvalue (Game|GetPlayerController 0))
  (EventDispatchers|UnbindEventfromBPonWidgetDeactivated (Variables|Default|GetWidget) (delegate Custom|BP_OnWidgetDeactivated_Event))
  (Utilities|IsValid _returnvalue
    (:Is%20Valid
      (Pawn|Possess _returnvalue (Variables|Default|GetOriginal%20Player%20Pawn))
      (Game|Player|SetViewTargetwithBlend _returnvalue (Variables|Default|GetOriginal%20Player%20Pawn) 0.3 "VTBlend_Linear" 0.0 true)
      (Collision|SetActorEnableCollision true))))

(event Input|EnhancedActionEvents|EnhancedInputActionIA_MoveUp
  (params (ActionValue :type Boolean) (ElapsedSeconds :type Float%20%28double-precision%29) (TriggeredSeconds :type Float%20%28double-precision%29) (InputAction :type Input%20Action%20Object%20Reference :default "/Game/Input/Actions/IA_MoveUp.IA_MoveUp"))
  (bind _ac_puzzleelement (Variables|Default|GetAC_PuzzleElement))
  (:Triggered
    (bind _value (Timeline|Lever%20Animation Play)
      (:Update
        (Transformation|SetRelativeRotation (Variables|Default|GetLever_Root) (Math|Rotator|MakeRotator 0.0 0.0 (Math|Float|Lerp 0.0 -6.2e+02 _value)) false false)
        (if (Variables|/Game/Blueprints/Interaction/AC_PuzzleElement.AC_PuzzleElement_C|GetSolved (Variables|Default|GetAC_PuzzleElement))
          (Collision|SetActorEnableCollision true)
          (if (Utilities|Operators|EqualEqual (Variables|/Script/Engine.SceneComponent|GetRelativeRotation (Variables|Default|GetLever_Root)) (Math|Rotator|MakeRotator 0.0 0.0 6.2e+02) 0.0)
            (Default|SetPuzzleSolved _ac_puzzleelement false)
            (Development|PrintString "Solved")
            (else
              (Default|SetPuzzleSolved _ac_puzzleelement false)
              (Development|PrintString "Not Solved")))))))
  (:Completed
    (Timeline|Lever%20Animation Stop)))

(event Input|EnhancedActionEvents|EnhancedInputActionIA_MoveDown
  (params (ActionValue :type Boolean) (ElapsedSeconds :type Float%20%28double-precision%29) (TriggeredSeconds :type Float%20%28double-precision%29) (InputAction :type Input%20Action%20Object%20Reference :default "/Game/Input/Actions/IA_MoveDown.IA_MoveDown"))
  (bind _ac_puzzleelement (Variables|Default|GetAC_PuzzleElement))
  (:Triggered
    (bind _value (Timeline|Lever%20Animation Reverse)
      (:Update
        (Transformation|SetRelativeRotation (Variables|Default|GetLever_Root) (Math|Rotator|MakeRotator 0.0 0.0 (Math|Float|Lerp 0.0 -6.2e+02 _value)) false false)
        (if (Variables|/Game/Blueprints/Interaction/AC_PuzzleElement.AC_PuzzleElement_C|GetSolved (Variables|Default|GetAC_PuzzleElement))
          (Collision|SetActorEnableCollision true)
          (if (Utilities|Operators|EqualEqual (Variables|/Script/Engine.SceneComponent|GetRelativeRotation (Variables|Default|GetLever_Root)) (Math|Rotator|MakeRotator 0.0 0.0 6.2e+02) 0.0)
            (Default|SetPuzzleSolved _ac_puzzleelement false)
            (Development|PrintString "Solved")
            (else
              (Default|SetPuzzleSolved _ac_puzzleelement false)
              (Development|PrintString "Not Solved")))))))
  (:Completed
    (Timeline|Lever%20Animation Stop)))

(event EventBeginPlay)

(event Collision|EventActorBeginOverlap
  (params (OtherActor :type Actor%20Object%20Reference)))

(event EventTick
  (params (DeltaSeconds :type Float%20%28single-precision%29)))

(event EventOnInteract
  (Variables|Default|SetOriginal%20Player%20Pawn (Game|Player|GetPlayerPawn 0))
  (Collision|SetActorEnableCollision false)
  (Game|Player|SetViewTargetwithBlend (Game|GetPlayerController 0) self 0.5 "VTBlend_Linear" 0.0 true)
  (Pawn|Possess (Game|GetPlayerController 0) self)
  (bind _returnvalue (Class|CommonActivatableWidgetContainerBase|AddWidget (Variables|/Game/UI/VM_HUD.VM_HUD_C|GetGameplay%20Overlay%20Stack (CallFunction|GetHUDVM)) "/Game/Blueprints/PossessPuzzle/UI_PossesPuzzleKeyboard.UI_PossesPuzzleKeyboard_C"))
  (bind _output_get (Variables|Default|SetWidget _returnvalue))
  (EventDispatchers|AssignBPonWidgetDeactivated _output_get (delegate Custom|BP_OnWidgetDeactivated_Event)))

(fn ConstructionScript
  (Components|Timeline|SetPlayRate (Variables|Default|GetLever%20Animation) (/ 1.0 (Variables|Default|GetAnimation%20Time%20In%20Seconds))))

(fn GetInteractionInfo
  (return "Crank"))