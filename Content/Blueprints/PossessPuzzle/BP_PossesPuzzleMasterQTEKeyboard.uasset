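; Possessable interactable for a keyboard button-mash QTE puzzle, shown to the player as "Shovel Snow".
; On interact it takes over possession and camera, pushes a QTE widget and starts a looping timer that drains the fill.
; X presses pulse and refill the bar; a full bar pauses the timer and plays the success animation.
; Widget deactivation returns possession and view to the original pawn; a fail event exists but is not called here.
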(event Custom|BP_OnWidgetDeactivated_Event
  (bind _returnvalue (Game|GetPlayerController 0))
  (EventDispatchers|UnbindEventfromBPonWidgetDeactivated (Variables|Default|GetWidget) (delegate Custom|BP_OnWidgetDeactivated_Event))
  (Utilities|IsValid _returnvalue
    (:Is%20Valid
      (Pawn|Possess _returnvalue (Variables|Default|GetOriginal%20Player%20Pawn))
      (Game|Player|SetViewTargetwithBlend _returnvalue (Variables|Default|GetOriginal%20Player%20Pawn) 0.3 "VTBlend_Linear" 0.0 true)
      (Collision|SetActorEnableCollision true))))

(event Custom|StartQTE
  (if (Utilities|Time|IsValidTimerHandle (Variables|Default|GetQTETimerHandle))
    (Utilities|Time|UnpauseTimerbyHandle (Variables|Default|GetQTETimerHandle))
    (else
      (bind _returnvalue (Utilities|Time|SetTimerbyEvent (delegate Custom|UpdateQTE) 0.01 true))
      (Variables|Default|SetQTETimerHandle _returnvalue)))
  (Default|SetFill (Variables|Default|GetWB_QTE) 0.0))

(event Custom|Hide%20Event
  (CallFunction|OnWidgetDeactivatedEvent))

(event Custom|QTEFail
  (bind _wb_qte (Variables|Default|GetWB_QTE))
  (bind _fail (Variables|/Game/UI/Puzzles/QTEs/UI_QTE_Range.UI_QTE_Range_C|GetFail _wb_qte))
  (Utilities|Time|PauseTimerbyHandle (Variables|Default|GetQTETimerHandle))
  (UserInterface|Animation|PlayAnimation _wb_qte _fail 0.0 1 "Forward" 1.0 true)
  (Class|UserWidget|BindtoAnimationFinished _wb_qte _fail (delegate Custom|Hide%20Event)))

(event Custom|UpdateQTE
  (bind _wb_qte (Variables|Default|GetWB_QTE))
  (bind _wb_qte_2 (Variables|Default|GetWB_QTE))
  (bind _rs_qte (Variables|/Game/UI/Puzzles/QTEs/UI_QTE_Range.UI_QTE_Range_C|GetRS_QTE _wb_qte_2))
  (bind _success (Variables|/Game/UI/Puzzles/QTEs/UI_QTE_Range.UI_QTE_Range_C|GetSuccess _wb_qte))
  (bind _returnvalue (Class|RadialSlider|GetValue _rs_qte))
  (if (< _returnvalue 1.0)
    (Default|SetFill (Variables|Default|GetWB_QTE) (- _returnvalue (Math|Float|Clamp(Float) (* (Variables|Default|GetDecay%20Per%20Second) 0.01))))
    (else
      (Utilities|Time|PauseTimerbyHandle (Variables|Default|GetQTETimerHandle))
      (UserInterface|Animation|PlayAnimation _wb_qte _success 0.0 1 "Forward" 1.0 true)
      (Class|UserWidget|BindtoAnimationFinished _wb_qte _success (delegate Custom|Hide%20Event)))))

(event EventBeginPlay)

(event Collision|EventActorBeginOverlap
  (params (OtherActor :type Actor%20Object%20Reference)))

(event EventTick
  (params (DeltaSeconds :type Float%20%28single-precision%29)))

(event EventOnInteract
  (Variables|Default|SetOriginal%20Player%20Pawn (Game|Player|GetPlayerPawn 0))
  (Collision|SetActorEnableCollision false)
  (Game|Player|SetViewTargetwithBlend (Game|GetPlayerController 0) self 0.5 "VTBlend_Linear" 0.0 true)
  (Pawn|Possess (Game|GetPlayerController 0) self)
  (CallFunction|StartQTE)
  (bind _returnvalue (Class|CommonActivatableWidgetContainerBase|AddWidget (Variables|/Game/UI/VM_HUD.VM_HUD_C|GetGameplay%20Overlay%20Stack (CallFunction|GetHUDVM)) "/Game/UI/Puzzles/QTEs/UI_QTE_Range.UI_QTE_Range_C"))
  (bind _output_get (Variables|Default|SetWidget _returnvalue))
  (EventDispatchers|AssignBPonWidgetDeactivated _output_get (delegate Custom|BP_OnWidgetDeactivated_Event)))

(event Input|KeyboardEvents|X
  (params (Key :type Key%20Structure :default "None"))
  (:Pressed
    (if (Widget|IsVisible (Variables|Default|GetWB_QTE))
      (CallFunction|QTEFill)
      (Development|PrintString "Hello"))))

(fn ConstructionScript)

(fn QTEFill
  (bind _wb_qte (Variables|Default|GetWB_QTE))
  (Utilities|FlowControl|Sequence
    (:then_0
      (Default|PlayPulse (Variables|Default|GetWB_QTE)))
    (:then_1
      (Default|SetFill _wb_qte (+ (Class|RadialSlider|GetValue (Variables|/Game/UI/Puzzles/QTEs/UI_QTE_Range.UI_QTE_Range_C|GetRS_QTE _wb_qte)) 0.1)))))

(fn GetInteractionInfo
  (return "Shovel Snow"))