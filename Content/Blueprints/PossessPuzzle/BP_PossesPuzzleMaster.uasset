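; Base interactable pawn for possession puzzles, offering an "Inspect" prompt and taking over player control when used.
; On interact it stores the player's pawn, disables its own collision, blends the view to itself, gets possessed and enables mouse interaction.
; It pushes the puzzle widget onto the HUD's gameplay overlay stack.
; When that widget deactivates, it restores the original pawn, view, input mode and collision.
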(event Custom|BP_OnWidgetDeactivated_Event
  (bind _returnvalue (Game|GetPlayerController 0))
  (EventDispatchers|UnbindEventfromBPonWidgetDeactivated (Variables|Default|GetWidget) (delegate Custom|BP_OnWidgetDeactivated_Event))
  (Utilities|IsValid _returnvalue
    (:Is%20Valid
      (Pawn|Possess _returnvalue (Variables|Default|GetOriginal%20Player%20Pawn))
      (Game|Player|SetViewTargetwithBlend _returnvalue (Variables|Default|GetOriginal%20Player%20Pawn) 0.5 "VTBlend_Linear" 0.0 true)
      (Variables|/Game/UI/VM_HUD.VM_HUD_C|SetUseMouseInteraction (CallFunction|GetHUDVM) false)
      (Collision|SetActorEnableCollision true))))

(event EventBeginPlay)

(event Collision|EventActorBeginOverlap
  (params (OtherActor :type Actor%20Object%20Reference)))

(event EventTick
  (params (DeltaSeconds :type Float%20%28single-precision%29)))

(event EventOnInteract
  (bind _hud_vm (CallFunction|GetHUDVM))
  (Variables|Default|SetOriginal%20Player%20Pawn (Game|Player|GetPlayerPawn 0))
  (Collision|SetActorEnableCollision false)
  (Game|Player|SetViewTargetwithBlend (Game|GetPlayerController 0) self 0.5 "VTBlend_Linear" 0.0 true)
  (Pawn|Possess (Game|GetPlayerController 0) self)
  (Variables|/Game/UI/VM_HUD.VM_HUD_C|SetUseMouseInteraction _hud_vm true)
  (bind _returnvalue (Class|CommonActivatableWidgetContainerBase|AddWidget (Variables|/Game/UI/VM_HUD.VM_HUD_C|GetGameplay%20Overlay%20Stack _hud_vm) "/Game/Blueprints/PossessPuzzle/UI_PossesPuzzle.UI_PossesPuzzle_C"))
  (bind _output_get (Variables|Default|SetWidget _returnvalue))
  (EventDispatchers|AssignBPonWidgetDeactivated _output_get (delegate Custom|BP_OnWidgetDeactivated_Event)))

(fn ConstructionScript)

(fn GetInteractionInfo
  (return "Inspect"))