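; BP_AllPuzzleChecker is an actor that watches a list of puzzle actors and reacts once all of them are solved.
; On BeginPlay it disables its collision, gathers each puzzle's AC_PuzzleElement component and binds to its solved-changed event.
; Each change rechecks every element; when all are solved it adds the "ReturnToStart" quest, enables collision and immediately quits the game.
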(event Custom|On%20Solved%20Changed_Event
  (params (is%20Solved :type Boolean))
  (bind _everyquestsolved (CallFunction|AllQuestsSolved))
  (if _everyquestsolved
    (CallFunction|AddQuest "ReturnToStart")
    (Collision|SetActorEnableCollision true)
    (Game|QuitGame 0 "Quit" false)))

(event EventBeginPlay
  (Collision|SetActorEnableCollision false)
  (for _array_element (Variables|Default|GetAllPuzzlesList)
    (Utilities|Array|Add (Variables|Default|GetPuzzleElement) (Actor|GetComponentbyClass _array_element "/Game/Blueprints/Interaction/AC_PuzzleElement.AC_PuzzleElement_C")))
  (for _array_element_2 (Variables|Default|GetPuzzleElement)
    (EventDispatchers|AssignOnSolvedChanged _array_element_2 (delegate Custom|On%20Solved%20Changed_Event))))

(event Collision|EventActorBeginOverlap
  (params (OtherActor :type Actor%20Object%20Reference)))

(event EventTick
  (params (DeltaSeconds :type Float%20%28single-precision%29)))

(fn ConstructionScript)

(fn AllQuestsSolved
  (for _array_element (Variables|Default|GetPuzzleElement)
    (if (not (Variables|/Game/Blueprints/Interaction/AC_PuzzleElement.AC_PuzzleElement_C|GetSolved _array_element))
      (return false)))
  (return true))